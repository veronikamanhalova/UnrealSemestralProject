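; Player ball Blueprint that creates the HUD, triggers the player's current ability and handles the end of the game.
; IA_Ability runs one ability at a time: Levitation raises the capsule in Flying mode, while Slowdown lowers global time dilation.
; Both revert after a Delay, with Slowdown's scaled by its factor to compensate for dilated time.
; EndMyGame shows the win widget, then quits shortly after.
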(event `self.ReceiveBeginPlay`
  (set `self.StartTransform` (`SceneComponent.K2_GetComponentToWorld` (`self.CapsuleComponent`)))
  (bind _returnvalue (`|CreateWidget` "/Game/UI/WBP_HUD.WBP_HUD_C" (`self.GetLocalViewingPlayerController`)))
  (`UserWidget.AddToViewport` _returnvalue 0)
  (set `self.UI` _returnvalue))

(event `EnhancedInput|/Game/Inputs/IA_Ability`
  (params (ActionValue :type Boolean) (ElapsedSeconds :type "Float (double-precision)") (TriggeredSeconds :type "Float (double-precision)") (InputAction :type "InputAction Object Reference" :default "/Game/Inputs/IA_Ability.IA_Ability"))
  (bind _capsulecomponent (`self.CapsuleComponent`))
  (bind (_returnvalue_x _returnvalue_y _returnvalue_z) (`KismetMathLibrary.BreakVector` (`SceneComponent.K2_GetComponentLocation` _capsulecomponent)))
  (:`Triggered`
    (if (and (`|EnumInequality` (`self.CurrentAbility`) "NewEnumerator0") (not (`self.IsAbilityActive`)))
      (set `self.IsAbilityActive` true)
      (set `self.ActiveAbility` (`self.CurrentAbility`))
      (switch `/Game/Enums/E_Ability` (`self.ActiveAbility`)
        (:`NewEnumerator1`
          ; Levitation
          (`CharacterMovementComponent.SetMovementMode` (`self.CharacterMovement`) "MOVE_Flying" 0)
          (`SceneComponent.K2_SetWorldLocation` _capsulecomponent (`KismetMathLibrary.MakeVector` _returnvalue_x _returnvalue_y (+ _returnvalue_z (`self.LevitationHeight`))) true false)
          (`KismetSystemLibrary.Delay` (`self.LevitationDuration`))
          (`CharacterMovementComponent.SetMovementMode` (`self.CharacterMovement`) "MOVE_Walking" 0)
          (set `self.IsAbilityActive` false)
          (set `self.ActiveAbility` "NewEnumerator0"))
        (:`NewEnumerator2`
          ; Slowdown
          (`GameplayStatics.SetGlobalTimeDilation` (`self.SlowdownFactor`))
          (set `self.CustomTimeDilation` 1.0)
          (`KismetSystemLibrary.Delay` (* (`self.SlowdownDuration`) (`self.SlowdownFactor`)))
          (`GameplayStatics.SetGlobalTimeDilation` 1.0)
          (set `self.CustomTimeDilation` 1.0)
          (set `self.IsAbilityActive` false)
          (set `self.ActiveAbility` "NewEnumerator0"))))))

(event `EndMyGame`
  ; End Game
  (bind _returnvalue (`|CreateWidget` "/Game/UI/WBP_Win.WBP_Win_C" (`self.GetLocalViewingPlayerController`)))
  (`UserWidget.AddToViewport` _returnvalue 0)
  (`KismetSystemLibrary.Delay` 2.0)
  (`KismetSystemLibrary.QuitGame` null "Quit"))

(fn `UserConstructionScript`)